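; Fake level exit actor that tricks the player into believing the level is over, then teleports the character to a set position.
; Overlapping the end trigger shows an end-level widget, waits, moves the character, reveals a hidden decal and shows a level-start widget.
; Both widgets are removed after a further delay.
; A separate particle trigger starts light trails and plays a reversed beam sound when the character overlaps it.
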(event OnComponentBeginOverlap(LevelEndTrigger)
  (params (OverlappedComponent :type Primitive%20Component%20Object%20Reference) (OtherActor :type Actor%20Object%20Reference) (OtherComp :type Primitive%20Component%20Object%20Reference) (OtherBodyIndex :type Integer) (bFromSweep :type Boolean) (SweepResult :type Hit%20Result%20Structure%20%28by%20ref%29))
  (bind _ascube_game_character (Utilities|Casting|CastToCubeGameCharacter OtherActor))
  (bind _returnvalue (UserInterface|CreateWidget "/Game/Blueprints/Level_Save_Checkpoint_Logic/LevelEndWidget.LevelEndWidget_C" 0 (Variables|Default|GetImageToEndLevel) (Variables|Default|GetTextTouchingTheFake)))
  (UserInterface|Viewport|AddtoViewport _returnvalue 0)
  (Utilities|FlowControl|Delay 4.0)
  (Transformation|SetActorLocation _ascube_game_character (Transformation|GetWorldLocation (Variables|Default|GetTeleportPosition)) false true)
  (Rendering|SetVisibility (Variables|Default|GetDecal) true false)
  (bind _returnvalue_2 (UserInterface|CreateWidget "/Game/Blueprints/Level_Save_Checkpoint_Logic/LevelStartWidget.LevelStartWidget_C" 0 (Variables|Default|GetImageToEndLevel) (Variables|Default|GetTextReappearing)))
  (UserInterface|Viewport|AddtoViewport _returnvalue_2 0)
  (Utilities|FlowControl|Delay 3.0)
  (Widget|RemovefromParent _returnvalue_2)
  (Widget|RemovefromParent _returnvalue))

(event OnComponentBeginOverlap(ParticleTrigger)
  (params (OverlappedComponent :type Primitive%20Component%20Object%20Reference) (OtherActor :type Actor%20Object%20Reference) (OtherComp :type Primitive%20Component%20Object%20Reference) (OtherBodyIndex :type Integer) (bFromSweep :type Boolean) (SweepResult :type Hit%20Result%20Structure%20%28by%20ref%29))
  (Utilities|Casting|CastToCubeGameCharacter OtherActor)
  (Effects|Particles|Trails|BeginTrails (Variables|Default|GetBlue_Lights_LvL_End) "None" "None" "ETrailWidthMode_FromCentre" 0.0)
  (Audio|SpawnSoundatLocation "/Game/Audio/Effekte/beam_effekt_reverse_Cue.beam_effekt_reverse_Cue" (.OutLocation (Actor|GetActorEyesViewPoint)) "0, 0, 0" 1.0 1.0 0.0 0 0))

(event EventBeginPlay
  (Rendering|SetVisibility (Variables|Default|GetDecal) false false))

(fn ConstructionScript)