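; FPS handles player death by restoring level and player state from the saved game.
; From BeginPlay it binds to the CubeGameCharacter's OnDestroyed event, which loads the SavePlayerProgress slot.
; Loading replaces all Transportable actors with ones spawned at saved cube transforms.
; It then spawns and possesses a new character with saved transform and inventory, and calls Respawn to rebind for the next death.
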(event Custom|SetUpLevel
  (params (Player%20Progress :type Save%20Player%20Progress%20Object%20Reference))
  ;[1 1 1] Set up Level after Death according to save file
  (bind _outactors (Actor|GetAllActorsOfClass "/Game/Cubes/Transportable.Transportable_C"))
  (for _array_element _outactors
    (Actor|DestroyActor _array_element))
  (for _array_element_2 (.cubepositions (Variables|/Game/Blueprints/Level_Save_Checkpoint_Logic/SavePlayerProgress.SavePlayerProgress_C|GetLevelState Player%20Progress))
    (Development|PrintString (Utilities|String|ToString(Transform) _array_element_2) true true "(R=0.000000,G=0.660000,B=1.000000,A=1.000000)" 1e+01)
    (Game|SpawnActorfromClass "/Game/Cubes/Transportable.Transportable_C" _array_element_2 "Undefined" 0 0)))

(event Custom|Respawn
  (bind _ascube_game_character (Utilities|Casting|CastToCubeGameCharacter (Game|GetPlayerCharacter 0)))
  (Game|BindEventtoOnDestroyed _ascube_game_character (delegate Custom|LoadSaveFile)))

(event Custom|SetUpPlayer
  (params (Player%20Progress :type Save%20Player%20Progress%20Object%20Reference))
  (bind _playerstate (Variables|/Game/Blueprints/Level_Save_Checkpoint_Logic/SavePlayerProgress.SavePlayerProgress_C|GetPlayerState Player%20Progress))
  ;[1 1 1] Set Up Player after death
  (bind _returnvalue (Game|SpawnActorfromClass "/Game/Blueprints/CubeGameCharacter.CubeGameCharacter_C" (.playerposition _playerstate) "Undefined" 0 0))
  (Variables|/Game/Blueprints/Items/InventoryComponent.InventoryComponent_C|SetInventory (Variables|/Game/Blueprints/CubeGameCharacter.CubeGameCharacter_C|GetInventoryComponent _returnvalue) (.playerinventory _playerstate))
  (Default|CallInventoryChangedDispatcher (Variables|/Game/Blueprints/CubeGameCharacter.CubeGameCharacter_C|GetInventoryComponent _returnvalue))
  (Pawn|Possess (Game|GetPlayerController 0) _returnvalue)
  (CallFunction|Respawn))

(event Custom|LoadSaveFile
  (params (DestroyedActor :type Actor%20Object%20Reference))
  (Development|PrintString "Try Load Savefile")
  (bind _returnvalue (SaveGame|LoadGamefromSlot (Variables|Default|GetGame%20Save%20Slot)))
  (bind _assave_player_progress (Utilities|Casting|CastToSavePlayerProgress _returnvalue))
  (CallFunction|SetUpLevel _assave_player_progress)
  (CallFunction|SetUpPlayer _assave_player_progress))

(event EventBeginPlay
  (bind _ascube_game_character (Utilities|Casting|CastToCubeGameCharacter (Game|GetPlayerCharacter 0)))
  (Game|BindEventtoOnDestroyed _ascube_game_character (delegate Custom|LoadSaveFile)))

(fn ConstructionScript)