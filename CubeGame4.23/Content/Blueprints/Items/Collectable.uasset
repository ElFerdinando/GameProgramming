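; Collectable item actor that the player picks up into their inventory.
; Interaction adds one unit of its item structure to the interactor's InventoryComponent and destroys the actor only if the add succeeds.
; While reported in interaction range, it enables custom depth on its mesh for a highlight, using a short restarting timer to switch it off once range notifications stop.
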(event Custom|TurnOffEmission
  (Variables|Default|SetTimer%20Running false)
  (Rendering|SetRenderCustomDepth (Variables|Default|GetStaticMesh) false))

(event EventBeginPlay)

(event EventIsinRangetoInteract
  (Rendering|SetRenderCustomDepth (Variables|Default|GetStaticMesh) true)
  (if (Variables|Default|GetTimer%20Running)
    (Utilities|Time|ClearandInvalidateTimerbyHandle (stale _returnvalue)))
  (bind _returnvalue (Utilities|Time|SetTimerbyEvent (delegate Custom|TurnOffEmission) 0.1))
  (Variables|Default|SetTimer%20Running true))

(event EventInteraction
  (params (Interactor :type Actor%20Object%20Reference))
  (bind _success (Default|AddtoInventory (Actor|GetComponentbyClass Interactor "/Game/Blueprints/Items/InventoryComponent.InventoryComponent_C") (Utilities|Struct|MakeSlotStructure (Variables|Default|GetCollectableStructure) 1)))
  (if _success
    (Actor|DestroyActor)))

(fn ConstructionScript)