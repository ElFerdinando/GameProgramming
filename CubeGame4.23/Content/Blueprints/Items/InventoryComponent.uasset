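; An actor component that stores a player's items in a fixed-size array of slot structures, sized on BeginPlay.
; Adding an item merges stackable items into the first slot of the same class without checking a stack limit, otherwise fills an empty slot.
; Each add fires an inventory-changed dispatcher and reports success unconditionally.
; Toggling creates or removes the inventory widget, placed at a set position on the player controller's HUD canvas.
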(event EventBeginPlay
  (CallFunction|PrepareInventory))

(fn ToggleInventory
  (Variables|Default|GetInventory%20Window
    (:then
      (Widget|RemovefromParent (Variables|Default|GetInventory%20Window))
      (Variables|Default|SetInventory%20Window 0))
    (:else
      (bind _returnvalue (UserInterface|CreateWidget "/Game/Blueprints/InventoryUI/InventoryWindow.InventoryWindow_C" 0 self))
      (Variables|Default|SetInventory%20Window _returnvalue)
      (bind _asmy_player_controller (Utilities|Casting|CastToMyPlayerController (Game|GetPlayerController 0)))
      (bind _returnvalue_2 (Class|CanvasPanel|AddChildtoCanvas (Variables|/Game/Blueprints/InventoryUI/HUD.HUD_C|GetHudCanvas (Variables|/Game/Blueprints/MyPlayerController.MyPlayerController_C|GetHudWidget _asmy_player_controller)) (Variables|Default|GetInventory%20Window)))
      (Class|CanvasPanelSlot|SetAutoSize _returnvalue_2 true)
      (Class|CanvasPanelSlot|SetAlignment _returnvalue_2 "(X=0.000000,Y=0.000000)")
      (Class|CanvasPanelSlot|SetAnchors _returnvalue_2 (Utilities|Struct|MakeAnchors "(X=0.000000,Y=0.000000)" "(X=0.000000,Y=0.000000)"))
      (Class|CanvasPanelSlot|SetPosition _returnvalue_2 (Variables|Default|GetPosition)))))

(fn AddtoInventory
  (params (ContentToAdd :type Slot%20Structure%20Structure))
  (if (.isstackable (.item ContentToAdd))
    (bind _stackindex (Utilities|HasPartialStack ContentToAdd)
      (:True
        (CallFunction|AddtoStack ContentToAdd _stackindex))
      (:False
        (CallFunction|CreateStack ContentToAdd :!label _label)))
    (else
      (goto _label)))
  (Default|CallInventoryChangedDispatcher)
  (return true))

(fn PrepareInventory
  (Utilities|Array|Resize (Variables|Default|GetInventory) (Variables|Default|GetNumberOfSlots)))

(fn CreateStack
  (params (ContentToAdd :type Slot%20Structure%20Structure))
  (bind _inventory (Variables|Default|GetInventory))
  (Utilities|Array|SetArrayElem _inventory (Utilities|Array|FindItem _inventory (Utilities|Struct|MakeSlotStructure "(Name_2_2CFFCA804AC053F35B7C15BFCE635073=NSLOCTEXT(\"\", \"30F97A4949514A1DC4380292675CAAC5\", \"None\"),isStackable_5_335F384D48820C666DE9DB8D786A2D99=True,Class_9_F1AE1F534E1B0D8FFAD33588CF592344=None,Thumbnail_13_16B20B764AC44C99B1ECF590CEA7CA36=None)")) ContentToAdd))

(fn AddtoStack
  (params (Slot%20Structure :type Slot%20Structure%20Structure) (SlotIndex :type Integer))
  (bind _inventory (Variables|Default|GetInventory))
  (bind _output (Utilities|Array|Get(acopy) _inventory SlotIndex))
  (Utilities|Array|SetArrayElem _inventory SlotIndex (Utilities|Struct|MakeSlotStructure (.item _output) (+ (.quantity _output) (.Quantity (Utilities|Struct|BreakSlotStructure Slot%20Structure))))))