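; FloatingObject is an actor that animates its static mesh with configurable movement and spinning.
; On BeginPlay it stores the start transform, adds optional world-axis offsets, and adds 360 degrees to each enabled rotation axis.
; The Movement timeline, at a configurable play rate, lerps location and each rotation component separately through two tracks, allowing full turns that a direct rotator interpolation would collapse.
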(event EventBeginPlay
  (bind _staticmesh (Variables|Default|GetStaticMesh))
  (Variables|Default|SetStartTransform (Transformation|GetWorldTransform _staticmesh))
  (Variables|Default|SetNewPosition (Transformation|GetWorldLocation _staticmesh))
  (Components|Timeline|SetPlayRate (Variables|Default|GetMovement) (Variables|Default|GetPlayrate))
  (if (Variables|Default|GetMove)
    (Variables|Default|SetNewPosition (Math|Vector|MakeVector (+ (.X (Math|Vector|BreakVector (Variables|Default|GetNewPosition))) (Variables|Default|GetForwardsMovement)) (+ (.Y (Math|Vector|BreakVector (Variables|Default|GetNewPosition))) (Variables|Default|GetSideWaysMovement)) (+ (.Z (Math|Vector|BreakVector (Variables|Default|GetNewPosition))) (Variables|Default|GetUpwardsMovement)))))
  (if (Variables|Default|GetTurnX)
    (Variables|Default|SetrotationX (+ (.roll (.rotation (Variables|Default|GetStartTransform))) 3.6e+02))
    (else
      (Variables|Default|SetrotationX (.roll (.rotation (Variables|Default|GetStartTransform))))))
  (if (Variables|Default|GetTurnY)
    (Variables|Default|SetrotationY (+ (.pitch (.rotation (Variables|Default|GetStartTransform))) 3.6e+02))
    (else
      (Variables|Default|SetrotationY (.pitch (.rotation (Variables|Default|GetStartTransform))))))
  (if (Variables|Default|GetTurnZ)
    (Variables|Default|SetrotationZ (+ (.yaw (.rotation (Variables|Default|GetStartTransform))) 3.6e+02))
    (bind (_direction _movement _rotation) (Timeline|Movement Play)
      (:Update
        (Transformation|SetWorldTransform (Variables|Default|GetStaticMesh) (Math|Transform|MakeTransform (Math|Vector|Lerp(Vector) (.location (Variables|Default|GetStartTransform)) (Variables|Default|GetNewPosition) _movement) (Math|Rotator|MakeRotator (Math|Float|Lerp (.roll (.rotation (Variables|Default|GetStartTransform))) (Variables|Default|GetrotationX) _rotation) (Math|Float|Lerp (.pitch (.rotation (Variables|Default|GetStartTransform))) (Variables|Default|GetrotationY) _rotation) (Math|Float|Lerp (.yaw (.rotation (Variables|Default|GetStartTransform))) (Variables|Default|GetrotationZ) _rotation)) "1,1,1") false false)))
    (else
      (Variables|Default|SetrotationZ (.yaw (.rotation (Variables|Default|GetStartTransform))))
      (Timeline|Movement Play))))

(fn ConstructionScript)