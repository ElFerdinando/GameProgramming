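; A switch-driven object that fades away and loses collision when its switch activates, then returns when it deactivates.
; On BeginPlay it registers with the switch and creates dynamic material instances for up to six slots.
; A timeline drives the Transparency parameter on those materials, playing forward to fade out and in reverse to restore.
; The construction script applies the configurable mesh, and collision toggles immediately as each fade starts.
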(event EventOnSwitchActivated
  (Collision|SetCollisionEnabled (Variables|Default|GetStaticMesh) "NoCollision")
  (bind _newtrack_0 (Timeline|FadeAway PlayFromStart)
    (:Update
      (for _array_element (Variables|Default|GetMaterials)
        (Rendering|Material|SetScalarParameterValue _array_element "Transparency" (Math|Float|Lerp 1.0 0.0 _newtrack_0) :!class /Script/Engine.MaterialInstanceDynamic)))))

(event EventOnSwitchDeactivated
  (Collision|SetCollisionEnabled (Variables|Default|GetStaticMesh) "QueryAndPhysics")
  (bind _newtrack_0 (Timeline|FadeAway ReverseFromEnd)
    (:Update
      (for _array_element (Variables|Default|GetMaterials)
        (Rendering|Material|SetScalarParameterValue _array_element "Transparency" (Math|Float|Lerp 1.0 0.0 _newtrack_0) :!class /Script/Engine.MaterialInstanceDynamic)))))

(event EventBeginPlay
  (CallFunction|ListentoSwitch)
  (bind _index (Utilities|FlowControl|ForLoopwithBreak 0 5 :!label _label)
    (:LoopBody
      (bind _returnvalue (Rendering|Material|CreateDynamicMaterialInstance (Variables|Default|GetStaticMesh) _index 0 "None" :!class /Script/Engine.PrimitiveComponent))
      (if (Utilities|IsValid _returnvalue)
        (Utilities|Array|SetArrayElem (Variables|Default|GetMaterials) _index _returnvalue)
        (else
          (goto _label Break))))))

(fn ConstructionScript
  (Components|StaticMesh|SetStaticMesh (Variables|Default|GetStaticMesh) (Variables|Default|GetMeshOfDisappearingObject)))