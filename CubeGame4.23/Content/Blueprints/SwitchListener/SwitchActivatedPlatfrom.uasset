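; A switch-listening platform that moves between its start position and an EndPoint marker when the switch toggles.
; BeginPlay registers with the switch, caches both world locations and sets the timeline play rate.
; Activation plays the Platform_Move timeline, lerping the platform with a swept move, and deactivation reverses it.
; Both switch events also print debug messages on screen.
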(event EventOnSwitchActivated
  (Development|PrintString "Platform got called On" true true "(R=0.000000,G=0.660000,B=1.000000,A=1.000000)" 5.0)
  (bind _newtrack_0 (Timeline|Platform_Move Play)
    (:Update
      (Transformation|SetWorldLocation (Variables|Default|GetPlatform) (Math|Vector|Lerp(Vector) (Variables|Default|GetStart_Location) (Variables|Default|GetEnd_Location) _newtrack_0) true false))))

(event EventOnSwitchDeactivated
  (Development|PrintString "Platform got called Off" true true "(R=0.000000,G=0.660000,B=1.000000,A=1.000000)" 5.0)
  (bind _newtrack_0 (Timeline|Platform_Move Reverse)
    (:Update
      (Transformation|SetWorldLocation (Variables|Default|GetPlatform) (Math|Vector|Lerp(Vector) (Variables|Default|GetStart_Location) (Variables|Default|GetEnd_Location) _newtrack_0) true false))))

(event EventBeginPlay
  (CallFunction|ListentoSwitch)
  (Variables|Default|SetStart_Location (Transformation|GetWorldLocation (Variables|Default|GetPlatform)))
  (Variables|Default|SetEnd_Location (Transformation|GetWorldLocation (Variables|Default|GetEnd_Point)))
  (Components|Timeline|SetPlayRate (Variables|Default|GetPlatform_Move) (Variables|Default|GetPlayrate)))

(fn ConstructionScript)