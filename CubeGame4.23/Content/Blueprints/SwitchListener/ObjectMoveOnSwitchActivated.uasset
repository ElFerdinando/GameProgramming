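; A switch-listening object that moves its static mesh between its starting position and an Endpoint component.
; On BeginPlay it registers with the switch, caches both world locations and applies a configurable play rate to the timeline.
; Activation plays the timeline, lerping the mesh with a swept move; deactivation stops it in place rather than reversing it.
; The construction script applies an optional mesh override.
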(event EventOnSwitchActivated
  (bind _newtrack_0 (Timeline|Platform_Move Play)
    (:Update
      (Transformation|SetWorldLocation (Variables|Default|GetStaticMesh) (Math|Vector|Lerp(Vector) (Variables|Default|GetStart_Location) (Variables|Default|GetEnd_Location) _newtrack_0) true false))))

(event EventOnSwitchDeactivated
  (bind _newtrack_0 (Timeline|Platform_Move Stop)
    (:Update
      (Transformation|SetWorldLocation (Variables|Default|GetStaticMesh) (Math|Vector|Lerp(Vector) (Variables|Default|GetStart_Location) (Variables|Default|GetEnd_Location) _newtrack_0) true false))))

(event EventBeginPlay
  (CallFunction|ListentoSwitch)
  (Variables|Default|SetStart_Location (Transformation|GetWorldLocation (Variables|Default|GetStaticMesh)))
  (Variables|Default|SetEnd_Location (Transformation|GetWorldLocation (Variables|Default|GetEndpoint)))
  (Components|Timeline|SetPlayRate (Variables|Default|GetPlatform_Move) (Variables|Default|GetPlayrate)))

(fn ConstructionScript
  (bind _staticmeshofobject (Variables|Default|GetStaticMeshOfObject))
  (if (Utilities|IsValid _staticmeshofobject)
    (Components|StaticMesh|SetStaticMesh (Variables|Default|GetStaticMesh) _staticmeshofobject)))