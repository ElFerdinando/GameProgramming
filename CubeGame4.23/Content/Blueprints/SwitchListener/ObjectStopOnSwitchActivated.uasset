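; Switch-listening moving object that travels between its start and an Endpoint until a switch activates, which stops it.
; A timeline, started at BeginPlay and on switch deactivation, lerps the swept mesh position at an adjustable play rate.
; Distance checks against the player camera drive a DoOnce that restarts the attached hover sound, which switch activation silences.
; The construction script applies an optional per-instance mesh.
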(event EventOnSwitchActivated
  (Audio|Components|Audio|Stop (Variables|Default|GetSound))
  (bind _newtrack_0 (Timeline|Platform_Move Stop)
    (:Update
      (Transformation|SetWorldLocation (Variables|Default|GetStaticMesh) (Math|Vector|Lerp(Vector) (Variables|Default|GetStart_Location) (Variables|Default|GetEnd_Location) _newtrack_0) true false)
      ;[1 1 1] Restart of Sound after to high distance
      (Math|Float|CompareFloat (Math|Vector|Distance(Vector) (Math|Vector|Lerp(Vector) (Variables|Default|GetStart_Location) (Variables|Default|GetEnd_Location) _newtrack_0) (Camera|GetCameraLocation (Game|GetPlayerCameraManager 0))) 9e+02
        (:>
          (goto _label Reset))
        (:<
          (Utilities|FlowControl|DoOnce true :!label _label
            (:Completed
              (Audio|Components|Audio|Play (Variables|Default|GetSound) 0.0))))))))

(event EventOnSwitchDeactivated
  (bind _newtrack_0 (Timeline|Platform_Move Play)
    (:Update
      (Transformation|SetWorldLocation (Variables|Default|GetStaticMesh) (Math|Vector|Lerp(Vector) (Variables|Default|GetStart_Location) (Variables|Default|GetEnd_Location) _newtrack_0) true false)
      ;[1 1 1] Restart of Sound after to high distance
      (Math|Float|CompareFloat (Math|Vector|Distance(Vector) (Math|Vector|Lerp(Vector) (Variables|Default|GetStart_Location) (Variables|Default|GetEnd_Location) _newtrack_0) (Camera|GetCameraLocation (Game|GetPlayerCameraManager 0))) 9e+02
        (:>
          (goto _label Reset))
        (:<
          (Utilities|FlowControl|DoOnce true :!label _label
            (:Completed
              (Audio|Components|Audio|Play (Variables|Default|GetSound) 0.0))))))))

(event EventBeginPlay
  (CallFunction|ListentoSwitch)
  (Variables|Default|SetStart_Location (Transformation|GetWorldLocation (Variables|Default|GetStaticMesh)))
  (Variables|Default|SetEnd_Location (Transformation|GetWorldLocation (Variables|Default|GetEndpoint)))
  (Components|Timeline|SetPlayRate (Variables|Default|GetPlatform_Move) (Variables|Default|GetPlayrate))
  (CallFunction|OnSwitchDeactivated)
  (bind _returnvalue (Audio|SpawnSoundAttached "/Game/Audio/Effekte/Hovering/hovering_cue.hovering_cue" (Variables|Default|GetStaticMesh) "None" "0, 0, 0" "0, 0, 0" "KeepRelativeOffset" false 1.0 1.0 0.0 0 0 false))
  (Variables|Default|SetSound _returnvalue)
  (Audio|Components|Audio|Stop (Variables|Default|GetSound)))

(fn ConstructionScript
  (bind _staticmeshofobject (Variables|Default|GetStaticMeshOfObject))
  (if (Utilities|IsValid _staticmeshofobject)
    (Components|StaticMesh|SetStaticMesh (Variables|Default|GetStaticMesh) _staticmeshofobject)))