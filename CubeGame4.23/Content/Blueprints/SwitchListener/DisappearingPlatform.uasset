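; Disappearing platform that turns non-solid and fades away when its linked switch activates, then returns when the switch deactivates.
; On BeginPlay it registers with the switch and creates dynamic material instances for six mesh material slots.
; Switch events toggle mesh collision immediately and play or reverse the FadeAway timeline, which drives the Transparency parameter on every instance.
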(event EventOnSwitchActivated
  (Collision|SetCollisionEnabled (Variables|Default|GetStaticMesh) "NoCollision")
  (bind _newtrack_0 (Timeline|FadeAway PlayFromStart)
    (:Update
      (for _array_element (Variables|Default|GetMaterials)
        (Rendering|Material|SetScalarParameterValue _array_element "Transparency" (Math|Float|Lerp 1.0 0.0 _newtrack_0) :!class /Script/Engine.MaterialInstanceDynamic)))))

(event EventOnSwitchDeactivated
  (Collision|SetCollisionEnabled (Variables|Default|GetStaticMesh) "QueryAndPhysics")
  (bind _newtrack_0 (Timeline|FadeAway ReverseFromEnd)
    (:Update
      (for _array_element (Variables|Default|GetMaterials)
        (Rendering|Material|SetScalarParameterValue _array_element "Transparency" (Math|Float|Lerp 1.0 0.0 _newtrack_0) :!class /Script/Engine.MaterialInstanceDynamic)))))

(event EventBeginPlay
  (CallFunction|ListentoSwitch)
  (for _index (range 0 5)
    (bind _returnvalue (Rendering|Material|CreateDynamicMaterialInstance (Variables|Default|GetStaticMesh) _index 0 "None" :!class /Script/Engine.PrimitiveComponent))
    (Utilities|Array|SetArrayElem (Variables|Default|GetMaterials) _index _returnvalue)))

(fn ConstructionScript)