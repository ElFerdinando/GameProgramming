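; SwitchListener is a parent Blueprint for objects that react to switches being activated or deactivated.
; ListenToSwitch finds actors tagged "Switch", casts them to Switch_Cube and asks each whether it matches this listener's SwitchID.
; Matching switches get their activated and deactivated events bound to OnSwitchActivated and OnSwitchDeactivated.
; Both handlers only print a debug message here, leaving the actual response to child classes.
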(event Custom|OnSwitchActivated
  ;[1 1 1] Listen to Switch
  ;;[1 1 1] Implementation in Child Class
  (Development|PrintString "Calling from Parrent"))

(event Custom|OnSwitchDeactivated
  ;[1 1 1] Listen to Switch
  ;;[1 1 1] Implementation in Child Class
  (Development|PrintString "Calling from Parrent"))

(event Custom|ListenToSwitch
  ;[1 1 1] Listen to Switch
  (Development|PrintString "See if there is Switch to listen" true true "(R=0.000000,G=0.660000,B=1.000000,A=1.000000)" 5.0)
  (bind _outactors (Actor|GetAllActorswithTag "Switch"))
  (for _array_element _outactors
    (Development|PrintString "found Switch by Tag" true true "(R=0.000000,G=0.660000,B=1.000000,A=1.000000)" 5.0)
    (bind _asswitch_cube (Utilities|Casting|CastToSwitch_Cube _array_element))
    (bind _result (Default|IsThisSwitch _asswitch_cube (Variables|Default|GetSwitch_ID)))
    (if _result
      (Development|PrintString "found Switch with Name")
      (EventDispatchers|BindEventtoSwitchActivated _asswitch_cube (delegate Custom|OnSwitchActivated))
      (EventDispatchers|BindEventtoSwitchDeactivated _asswitch_cube (delegate Custom|OnSwitchDeactivated))
      (else
        (Development|PrintString "Switch has another Name" true true "(R=0.000000,G=0.660000,B=1.000000,A=1.000000)" 5.0)))))

(fn ConstructionScript)