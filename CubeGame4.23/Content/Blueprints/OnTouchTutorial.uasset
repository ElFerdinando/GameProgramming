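; Trigger actor that shows a tutorial widget on screen when its trigger volume is first overlapped.
; On overlap, a DoOnce creates a Tutorials widget for player 0, passes it the ImagesToShowInTutorial variable and adds it to the viewport.
; The overlapping actor is not filtered, so any overlap can use up the single showing.
; The construction script applies ResizeTrigger as the volume's world scale, keeping its location and rotation.
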(event OnComponentBeginOverlap(TriggerVolume)
  (params (OverlappedComponent :type Primitive%20Component%20Object%20Reference) (OtherActor :type Actor%20Object%20Reference) (OtherComp :type Primitive%20Component%20Object%20Reference) (OtherBodyIndex :type Integer) (bFromSweep :type Boolean) (SweepResult :type Hit%20Result%20Structure%20%28by%20ref%29))
  (Utilities|FlowControl|DoOnce false
    (:Completed
      (bind _returnvalue (UserInterface|CreateWidget "/Game/UI/Tutorials.Tutorials_C" (Game|GetPlayerController 0) (Variables|Default|GetImagesToShowInTutorial)))
      (UserInterface|Viewport|AddtoViewport _returnvalue 0))))

(event EventBeginPlay)

(event Collision|EventActorBeginOverlap
  (params (OtherActor :type Actor%20Object%20Reference)))

(fn ConstructionScript
  (bind _triggervolume (Variables|Default|GetTriggerVolume))
  (Transformation|SetWorldTransform _triggervolume (Math|Transform|MakeTransform (Transformation|GetWorldLocation _triggervolume) (Transformation|GetWorldRotation _triggervolume) (Variables|Default|GetResizeTrigger)) false false))