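; Rook-style actor that slides along its right or forward axis when a CubeGameCharacter enters its line of detection.
; The construction script sizes and offsets axis-aligned trigger volumes by Range.
; While idle, Tick checks those volumes in priority order and picks a signed target scaled by Range and actor scale.
; The Movement timeline lerps the mesh there without sweep, blocking new checks until it finishes.
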(event EventBeginPlay
  (Components|Timeline|SetPlayRate (Variables|Default|GetMovement) (Variables|Default|GetPlayrate)))

(event EventTick
  (params (DeltaSeconds :type Float%20%28single-precision%29))
  (bind _returnvalue (Transformation|GetActorScale3D))
  (bind _staticmesh (Variables|Default|GetStaticMesh))
  (bind _staticmesh_2 (Variables|Default|GetStaticMesh))
  (bind __y (Variables|Default|Get+Y))
  (bind __y_2 (Variables|Default|Get-Y))
  (bind __x (Variables|Default|Get+X))
  (bind __x_2 (Variables|Default|Get-X))
  (bind _staticmesh_3 (Variables|Default|GetStaticMesh))
  (bind _staticmesh_4 (Variables|Default|GetStaticMesh))
  (bind _staticmesh_5 (Variables|Default|GetStaticMesh))
  (bind (_x _y) (Math|Vector|BreakVector _returnvalue))
  (if (not (Variables|Default|GetIsAlreadyMoving))
    (bind _returnvalue_2 (Collision|ComponentOverlapActors __y (Transformation|GetWorldTransform __y) (Utilities|Array|MakeArray "ObjectTypeQuery3") "/Game/Blueprints/CubeGameCharacter.CubeGameCharacter_C"))
    (if _returnvalue_2
      (Variables|Default|SetNewPosition (+ (* (* (* (Math|Vector|GetRightVector _staticmesh_4) (Variables|Default|GetRange)) 50) _y) (Transformation|GetWorldLocation _staticmesh_4)))
      (Variables|Default|SetIsAlreadyMoving true :!label _label)
      (bind _position (Timeline|Movement PlayFromStart)
        (:Update
          (Transformation|SetWorldLocation _staticmesh_3 (Math|Vector|Lerp(Vector) (Transformation|GetWorldLocation _staticmesh_3) (Variables|Default|GetNewPosition) _position) false false))
        (:Finished
          (Variables|Default|SetIsAlreadyMoving false)))
      (else
        (bind _returnvalue_3 (Collision|ComponentOverlapActors __y_2 (Transformation|GetWorldTransform __y_2) (Utilities|Array|MakeArray "ObjectTypeQuery3") "/Game/Blueprints/CubeGameCharacter.CubeGameCharacter_C"))
        (if _returnvalue_3
          (Variables|Default|SetNewPosition (+ (* (* (* (Math|Vector|GetRightVector _staticmesh_2) (Variables|Default|GetRange)) -50) _y) (Transformation|GetWorldLocation _staticmesh_2)))
          (goto _label)
          (else
            (bind _returnvalue_4 (Collision|ComponentOverlapActors __x (Transformation|GetWorldTransform __x) (Utilities|Array|MakeArray "ObjectTypeQuery3") "/Game/Blueprints/CubeGameCharacter.CubeGameCharacter_C"))
            (if _returnvalue_4
              (Variables|Default|SetNewPosition (+ (* (* (* (Math|Vector|GetForwardVector _staticmesh) (Variables|Default|GetRange)) 50) _x) (Transformation|GetWorldLocation _staticmesh)))
              (goto _label)
              (else
                (bind _returnvalue_5 (Collision|ComponentOverlapActors __x_2 (Transformation|GetWorldTransform __x_2) (Utilities|Array|MakeArray "ObjectTypeQuery3") "/Game/Blueprints/CubeGameCharacter.CubeGameCharacter_C"))
                (if _returnvalue_5
                  (Variables|Default|SetNewPosition (+ (* (* (* (Math|Vector|GetForwardVector _staticmesh_5) (Variables|Default|GetRange)) -50) _x) (Transformation|GetWorldLocation _staticmesh_5)))
                  (goto _label))))))))))

(fn ConstructionScript
  (bind _range (Variables|Default|GetRange))
  (bind _range_2 (Variables|Default|GetRange))
  (bind _range_3 (Variables|Default|GetRange))
  (bind _range_4 (Variables|Default|GetRange))
  (Transformation|SetRelativeTransform (Variables|Default|Get+Y) (Math|Transform|MakeTransform (Math|Vector|MakeVector 0.0 (* _range 25.0) 4e+01) "0, 0, 0" (Math|Vector|MakeVector 1.0 _range 1.0)) false false)
  (Transformation|SetRelativeTransform (Variables|Default|Get-Y) (Math|Transform|MakeTransform (Math|Vector|MakeVector 0.0 (* _range_4 -25.0) 4e+01) "0, 0, 0" (Math|Vector|MakeVector 1.0 _range_4 1.0)) false false)
  (Transformation|SetRelativeTransform (Variables|Default|Get+X) (Math|Transform|MakeTransform (Math|Vector|MakeVector (* _range_3 25.0) 0.0 4e+01) "0, 0, 0" (Math|Vector|MakeVector _range_3 1.0 1.0)) false false)
  (Transformation|SetRelativeTransform (Variables|Default|Get-X) (Math|Transform|MakeTransform (Math|Vector|MakeVector (* _range_2 -25.0) 0.0 4e+01) "0, 0, 0" (Math|Vector|MakeVector _range_2 1.0 1.0)) false false))