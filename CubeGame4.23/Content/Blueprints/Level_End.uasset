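; Level end actor that finishes the current level when the CubeGameCharacter enters its trigger and loads the chosen next level.
; The end trigger shows a LevelEndWidget with configurable image and text, then flags the matching level as reached in the LevelsReached save game.
; After a short delay it opens the level named by the NextLevel enum.
; A separate particle trigger starts the blue light trails and plays a beam sound.
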(event OnComponentBeginOverlap(LevelEndTrigger)
  (params (OverlappedComponent :type Primitive%20Component%20Object%20Reference) (OtherActor :type Actor%20Object%20Reference) (OtherComp :type Primitive%20Component%20Object%20Reference) (OtherBodyIndex :type Integer) (bFromSweep :type Boolean) (SweepResult :type Hit%20Result%20Structure%20%28by%20ref%29))
  (Utilities|Casting|CastToCubeGameCharacter OtherActor)
  (bind _returnvalue (UserInterface|CreateWidget "/Game/Blueprints/Level_Save_Checkpoint_Logic/LevelEndWidget.LevelEndWidget_C" 0 (Variables|Default|GetImageToEndLevel) (Variables|Default|GetTextToEndLevel)))
  (UserInterface|Viewport|AddtoViewport _returnvalue 0)
  (bind _returnvalue_2 (SaveGame|LoadGamefromSlot (Variables|Default|GetLevelReachedSavefile)))
  (bind _aslevels_reached (Utilities|Casting|CastToLevelsReached _returnvalue_2))
  (switch Utilities|FlowControl|Switch|SwitchonLevellist (Variables|Default|GetNext%20Level)
    (:NewEnumerator0
      (Variables|/Game/Blueprints/Level_Save_Checkpoint_Logic/LevelsReached.LevelsReached_C|SetLevel1Reached _aslevels_reached true))
    (:NewEnumerator1
      (Variables|/Game/Blueprints/Level_Save_Checkpoint_Logic/LevelsReached.LevelsReached_C|SetLevel2Reached _aslevels_reached true))
    (:NewEnumerator5
      (Variables|/Game/Blueprints/Level_Save_Checkpoint_Logic/LevelsReached.LevelsReached_C|SetLevel3Reached _aslevels_reached true)))
  (SaveGame|SaveGametoSlot _aslevels_reached (Variables|Default|GetLevelReachedSavefile))
  (Utilities|FlowControl|Delay 4.0)
  (Game|OpenLevel(byName) (Utilities|String|StringToName (Utilities|String|EnumtoString (Variables|Default|GetNext%20Level)))))

(event OnComponentBeginOverlap(ParticleTrigger)
  (params (OverlappedComponent :type Primitive%20Component%20Object%20Reference) (OtherActor :type Actor%20Object%20Reference) (OtherComp :type Primitive%20Component%20Object%20Reference) (OtherBodyIndex :type Integer) (bFromSweep :type Boolean) (SweepResult :type Hit%20Result%20Structure%20%28by%20ref%29))
  (Utilities|Casting|CastToCubeGameCharacter OtherActor)
  (Effects|Particles|Trails|BeginTrails (Variables|Default|GetBlue_Lights_LvL_End) "None" "None" "ETrailWidthMode_FromCentre" 0.0)
  (Audio|SpawnSoundatLocation "/Game/Audio/Effekte/beam_effekt_reverse_Cue.beam_effekt_reverse_Cue" (.OutLocation (Actor|GetActorEyesViewPoint)) "0, 0, 0" 1.0 1.0 0.0 0 0))

(fn ConstructionScript)