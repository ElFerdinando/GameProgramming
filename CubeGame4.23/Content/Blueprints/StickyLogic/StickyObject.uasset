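; StickyObject is a cube with configurable sticky faces that the player can attach cubes from their inventory to.
; CanPlaceCube maps the hit to a local face, derives the neighboring transform and sweeps PlayerTouchTest there to reject spots overlapping a character.
; Valid targets briefly enable custom depth as a highlight, cleared by a restarting timer.
; Placement spawns the first inventory item at the character and lerps it into position by timeline, with success or failure sounds.
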(event Custom|TurnOffEmission
  ;[1 1 1] Is Is Range
  (Rendering|SetRenderCustomDepth (Variables|Default|GetStaticMesh) false))

(event EventIsinRangetoPlace
  (params (HitLocation :type Vector :default "0, 0, 0"))
  ;[1 1 1] Is Is Range
  (bind _sucess (Utilities|CanPlaceCube HitLocation)
    (:Return
      (if _sucess
        (Rendering|SetRenderCustomDepth (Variables|Default|GetStaticMesh) true)
        (if (Variables|Default|GetTimerRunning)
          (Utilities|Time|ClearandInvalidateTimerbyHandle (stale _returnvalue)))
        (bind _returnvalue (Utilities|Time|SetTimerbyEvent (delegate Custom|TurnOffEmission) 0.1))
        (Variables|Default|SetTimerRunning true)))))

(event EventTryPlacingCube
  (params (HitLocation :type Vector :default "0, 0, 0") (CharacterToTakeCubeFrom :type Cube%20Game%20Character%20Object%20Reference))
  ;[1 1 1] CubePlacement
  (Variables|Default|SetCharacter CharacterToTakeCubeFrom)
  (bind _sucess (Utilities|CanPlaceCube HitLocation)
    (:Return
      (if _sucess
        (Audio|SpawnSound2D "/Game/Audio/Effekte/Block_anstecken_Cue.Block_anstecken_Cue" 1.0 1.0 0.0 0)
        (bind _returnvalue (Game|SpawnActorfromClass (.class (.Item (Utilities|Struct|BreakSlotStructure (Utilities|Array|Get(acopy) (Variables|/Game/Blueprints/Items/InventoryComponent.InventoryComponent_C|GetInventory (Variables|/Game/Blueprints/CubeGameCharacter.CubeGameCharacter_C|GetInventoryComponent (Variables|Default|GetCharacter))))))) (Math|Transform|MakeTransform (Transformation|GetWorldLocation (Variables|/Script/Engine.Actor|GetRootComponent (Variables|Default|GetCharacter))) (.rotation (Variables|Default|GetTransformToPlace)) "1,1,1") "Undefined" 0 0))
        (Default|RemoveSingleItem (Variables|Default|GetCharacter))
        (bind _newtrack_0 (Timeline|CubeMovement PlayFromStart)
          (:Update
            (Transformation|SetWorldLocation (Variables|/Script/Engine.Actor|GetRootComponent _returnvalue) (Math|Vector|Lerp(Vector) (Transformation|GetWorldLocation (Variables|/Script/Engine.Actor|GetRootComponent _returnvalue)) (.location (Variables|Default|GetTransformToPlace)) _newtrack_0) true false)))
        (else
          (Audio|SpawnSound2D "/Game/Audio/Effekte/Block_connect_fail_Cue.Block_connect_fail_Cue" 1.0 1.0 0.0 0))))))

(fn ConstructionScript)