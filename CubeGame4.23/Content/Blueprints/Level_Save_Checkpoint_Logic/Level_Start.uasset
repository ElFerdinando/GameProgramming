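; Level start actor that shows a level intro widget and creates or restores the player's checkpoint save on BeginPlay.
; A save matching the current level respawns Transportable cubes and restores player position and inventory, then plays a beam sound and trail effect.
; Otherwise it saves the level name, cube transforms, player inventory and its own transform as player position to the SavePlayerProgress slot.
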(event Custom|SaveLevelState
  (params (PlayerProgress :type Save%20Player%20Progress%20Object%20Reference))
  (bind _temporaryarray (Variables|Default|GettemporaryArray))
  ;[1 1 1] Save Level State
  (Utilities|Array|Clear (Variables|Default|GettemporaryArray))
  (bind _outactors (Actor|GetAllActorsOfClass "/Game/Cubes/Transportable.Transportable_C"))
  (for _array_element _outactors
    (Utilities|Array|Add _temporaryarray (Transformation|GetActorTransform _array_element)))
  (Development|PrintString "Array ready")
  (Variables|/Game/Blueprints/Level_Save_Checkpoint_Logic/SavePlayerProgress.SavePlayerProgress_C|SetLevelState PlayerProgress (Utilities|Struct|MakeLevelState (Utilities|String|EnumtoString (Variables|Default|GetCurrent%20Level)) _temporaryarray)))

(event Custom|SavePlayerState
  (params (Player%20Progress :type Save%20Player%20Progress%20Object%20Reference))
  ;[1 1 1] Save Player State
  (bind _ascube_game_character (Utilities|Casting|CastToCubeGameCharacter (Game|GetPlayerCharacter 0)))
  (Variables|/Game/Blueprints/Level_Save_Checkpoint_Logic/SavePlayerProgress.SavePlayerProgress_C|SetPlayerState Player%20Progress (Utilities|Struct|MakePlayerState (Transformation|GetActorTransform) (Variables|/Game/Blueprints/Items/InventoryComponent.InventoryComponent_C|GetInventory (Variables|/Game/Blueprints/CubeGameCharacter.CubeGameCharacter_C|GetInventoryComponent _ascube_game_character)))))

(event Custom|LoadPlayerState
  (params (Player%20Progress :type Save%20Player%20Progress%20Object%20Reference))
  (bind _playerstate (Variables|/Game/Blueprints/Level_Save_Checkpoint_Logic/SavePlayerProgress.SavePlayerProgress_C|GetPlayerState Player%20Progress))
  ;[1 1 1] Load Player State
  (bind _ascube_game_character (Utilities|Casting|CastToCubeGameCharacter (Game|GetPlayerCharacter 0)))
  (Transformation|SetActorTransform _ascube_game_character (.playerposition _playerstate) false true)
  (Variables|/Game/Blueprints/Items/InventoryComponent.InventoryComponent_C|SetInventory (Variables|/Game/Blueprints/CubeGameCharacter.CubeGameCharacter_C|GetInventoryComponent _ascube_game_character) (.playerinventory _playerstate))
  (Default|ToggleInventory (Variables|/Game/Blueprints/CubeGameCharacter.CubeGameCharacter_C|GetInventoryComponent _ascube_game_character))
  (Default|CallInventoryChangedDispatcher (Variables|/Game/Blueprints/CubeGameCharacter.CubeGameCharacter_C|GetInventoryComponent _ascube_game_character)))

(event Custom|LoadLevelState
  (params (Player%20Progress :type Save%20Player%20Progress%20Object%20Reference))
  ;[1 1 1] Load Level State
  (bind _outactors (Actor|GetAllActorswithTag "Transportable"))
  (for _array_element _outactors
    (Actor|DestroyActor _array_element))
  (for _array_element_2 (.cubepositions (Variables|/Game/Blueprints/Level_Save_Checkpoint_Logic/SavePlayerProgress.SavePlayerProgress_C|GetLevelState Player%20Progress))
    (Game|SpawnActorfromClass "/Game/Cubes/Transportable.Transportable_C" _array_element_2 "Undefined" 0 0)))

(event EventBeginPlay
  ;[1 1 1] Create/Load Savefile
  (bind _returnvalue (UserInterface|CreateWidget "/Game/Blueprints/Level_Save_Checkpoint_Logic/LevelStartWidget.LevelStartWidget_C" 0 (Variables|Default|GetStartLevelImage) (Variables|Default|GetStartLevelText)))
  (UserInterface|Viewport|AddtoViewport _returnvalue 0)
  (bind _returnvalue_2 (SaveGame|DoesSaveGameExist (Variables|Default|GetGameSave_Slot)))
  (if _returnvalue_2
    (bind _returnvalue_3 (SaveGame|LoadGamefromSlot (Variables|Default|GetGameSave_Slot)))
    (bind _output_get (Variables|Default|SetsavePlayerSubclass _returnvalue_3))
    (bind _assave_player_progress (Utilities|Casting|CastToSavePlayerProgress _output_get))
    (if (Utilities|Enum|Equal(Enum) (.levelname (Variables|/Game/Blueprints/Level_Save_Checkpoint_Logic/SavePlayerProgress.SavePlayerProgress_C|GetLevelState _assave_player_progress)) (Utilities|String|EnumtoString (Variables|Default|GetCurrent%20Level)))
      (CallFunction|LoadLevelState _assave_player_progress)
      (CallFunction|LoadPlayerState _assave_player_progress)
      (Development|PrintString "Load Checkpoint")
      (Utilities|FlowControl|RetriggerableDelay 1.5)
      (Audio|SpawnSound2D "/Game/Audio/Effekte/beam_effekt_Cue.beam_effekt_Cue" 1.0 1.0 0.0 0)
      (Utilities|FlowControl|RetriggerableDelay 0.7)
      (Effects|Particles|Trails|BeginTrails (Variables|Default|GetBlue_Lights_LvL_Start) "None" "None" "ETrailWidthMode_FromCentre" 0.0)
      (else
        (CallFunction|SaveLevelState _assave_player_progress)
        (CallFunction|SavePlayerState _assave_player_progress)
        (SaveGame|SaveGametoSlot _assave_player_progress (Variables|Default|GetGameSave_Slot))))
    (else
      (bind _returnvalue_4 (SaveGame|CreateSaveGameObject "/Game/Blueprints/Level_Save_Checkpoint_Logic/SavePlayerProgress.SavePlayerProgress_C"))
      (bind _output_get_2 (Variables|Default|SetsavePlayerSubclass _returnvalue_4))
      (bind _assave_player_progress_2 (Utilities|Casting|CastToSavePlayerProgress _output_get_2))
      (CallFunction|SaveLevelState _assave_player_progress_2)
      (CallFunction|SavePlayerState _assave_player_progress_2)
      (SaveGame|SaveGametoSlot _assave_player_progress_2 (Variables|Default|GetGameSave_Slot))
      (Development|PrintString "Save Start of Level"))))

(fn ConstructionScript)