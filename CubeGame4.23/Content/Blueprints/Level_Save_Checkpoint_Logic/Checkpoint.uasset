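; Checkpoint actor that saves game progress when an actor tagged Player overlaps its resizable trigger box, with particle, sound and on-screen feedback.
; It loads the existing SavePlayerProgress slot, overwrites player and level state, then writes it back, doing nothing if the load fails.
; Player state holds the checkpoint's spawn transform and inventory; level state holds the level name and all Transportable transforms.
; A timeline bobs and spins the mesh.
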(event OnComponentBeginOverlap(SaveTriggerVolume)
  (params (OverlappedComponent :type Primitive%20Component%20Object%20Reference) (OtherActor :type Actor%20Object%20Reference) (OtherComp :type Primitive%20Component%20Object%20Reference) (OtherBodyIndex :type Integer) (bFromSweep :type Boolean) (SweepResult :type Hit%20Result%20Structure%20%28by%20ref%29))
  ;[1 1 1] Save At Checkpoint
  (if (Actor|ActorHasTag OtherActor "Player")
    (bind _returnvalue (SaveGame|LoadGamefromSlot (Variables|Default|GetGameSave_Slot)))
    (bind _output_get (Variables|Default|SetsavePlayerSubclass _returnvalue))
    (bind _assave_player_progress (Utilities|Casting|CastToSavePlayerProgress _output_get))
    (CallFunction|SavePlayerState _assave_player_progress)
    (CallFunction|SaveLevelState _assave_player_progress)
    (SaveGame|SaveGametoSlot _assave_player_progress (Variables|Default|GetGameSave_Slot))
    ;[1 1 1] Partickle Effekt
    (Effects|Particles|Trails|BeginTrails (Variables|Default|GetGreen_Explotion_Save_Event) "None" "None" "ETrailWidthMode_FromCentre" 0.0)
    (Audio|SpawnSoundatLocation "/Game/Audio/Effekte/Sparks_Checkpoint_Cue.Sparks_Checkpoint_Cue" "0, 0, 0" "0, 0, 0" 1.0 1.0 0.0 0 0)
    (Development|PrintString "Saved at Checkpoint")
    (Development|PrintString "At Position")
    (Development|PrintString (Utilities|String|ToString(Transform) (.playerposition (Variables|/Game/Blueprints/Level_Save_Checkpoint_Logic/SavePlayerProgress.SavePlayerProgress_C|GetPlayerState _assave_player_progress))))))

(event Custom|SaveLevelState
  (params (PlayerProgress :type Save%20Player%20Progress%20Object%20Reference))
  (bind _temporaryarray (Variables|Default|GettemporaryArray))
  ;[1 1 1] Save Level State
  (Utilities|Array|Clear (Variables|Default|GettemporaryArray))
  (bind _outactors (Actor|GetAllActorsOfClass "/Game/Cubes/Transportable.Transportable_C"))
  (for _array_element _outactors
    (Utilities|Array|Add _temporaryarray (Transformation|GetActorTransform _array_element)))
  (Variables|/Game/Blueprints/Level_Save_Checkpoint_Logic/SavePlayerProgress.SavePlayerProgress_C|SetLevelState PlayerProgress (Utilities|Struct|MakeLevelState (Utilities|String|EnumtoString (Variables|Default|GetSave%20Current%20Level)) _temporaryarray)))

(event Custom|SavePlayerState
  (params (Player%20Progress :type Save%20Player%20Progress%20Object%20Reference))
  ;[1 1 1] Save Player State
  (bind _ascube_game_character (Utilities|Casting|CastToCubeGameCharacter (Game|GetPlayerCharacter 0)))
  (Variables|/Game/Blueprints/Level_Save_Checkpoint_Logic/SavePlayerProgress.SavePlayerProgress_C|SetPlayerState Player%20Progress (Utilities|Struct|MakePlayerState (Variables|Default|GetPlayerSpawnTransform) (Variables|/Game/Blueprints/Items/InventoryComponent.InventoryComponent_C|GetInventory (Variables|/Game/Blueprints/CubeGameCharacter.CubeGameCharacter_C|GetInventoryComponent _ascube_game_character))))
  (Default|CallInventoryChangedDispatcher (Variables|/Game/Blueprints/CubeGameCharacter.CubeGameCharacter_C|GetInventoryComponent _ascube_game_character)))

(event EventBeginPlay
  ;[1 1 1] Set Player Spawn Position of Checkpoint
  (Variables|Default|SetPlayerSpawnTransform (Math|Transform|MakeTransform (Transformation|GetWorldLocation (Variables|Default|GetSpawnLocation)) (.rotation (Transformation|GetActorTransform)) "1,1,1"))
  (Variables|Default|SetStartTransform (Transformation|GetWorldTransform (Variables|Default|GetStaticMesh)))
  (bind (_direction _movement _rotation) (Timeline|CheckpointAnimation Play)
    (:Update
      (Transformation|SetWorldTransform (Variables|Default|GetStaticMesh) (Math|Transform|MakeTransform (Math|Vector|MakeVector (.X (Math|Vector|BreakVector (.location (Variables|Default|GetStartTransform)))) (.Y (Math|Vector|BreakVector (.location (Variables|Default|GetStartTransform)))) (Math|Float|Lerp (.Z (Math|Vector|BreakVector (.location (Variables|Default|GetStartTransform)))) (+ (.Z (Math|Vector|BreakVector (.location (Variables|Default|GetStartTransform)))) 5e+01) _movement)) (Math|Rotator|MakeRotator (.Roll (Math|Rotator|BreakRotator (.rotation (Variables|Default|GetStartTransform)))) (.Pitch (Math|Rotator|BreakRotator (.rotation (Variables|Default|GetStartTransform)))) (Math|Float|Lerp (.Yaw (Math|Rotator|BreakRotator (.rotation (Variables|Default|GetStartTransform)))) (+ (.Yaw (Math|Rotator|BreakRotator (.rotation (Variables|Default|GetStartTransform)))) 3.6e+02) _rotation)) "1,1,1") false false))))

(fn ConstructionScript
  (Components|Box|SetBoxExtent (Variables|Components|GetSaveTriggerVolume) (Variables|Default|GetResizeTriggerVolume) true))