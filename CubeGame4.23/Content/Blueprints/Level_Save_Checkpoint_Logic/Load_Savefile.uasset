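; Trigger-volume actor that loads saved player progress when the CubeGameCharacter overlaps it.
; It reads the SavePlayerProgress slot, opens the saved level, then immediately replaces tagged Transportable actors with spawns at saved cube transforms.
; It also restores the player's transform and inventory and fires the inventory-changed dispatcher, all in the same call chain as OpenLevel.
; The construction script sizes the trigger box from ResizeTriggerVolume.
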(event OnComponentBeginOverlap(OpenTrigger)
  (params (OverlappedComponent :type Primitive%20Component%20Object%20Reference) (OtherActor :type Actor%20Object%20Reference) (OtherComp :type Primitive%20Component%20Object%20Reference) (OtherBodyIndex :type Integer) (bFromSweep :type Boolean) (SweepResult :type Hit%20Result%20Structure%20%28by%20ref%29))
  ;[1 1 1] open save file on touch
  (Utilities|Casting|CastToCubeGameCharacter OtherActor)
  (CallFunction|LoadGameSave))

(event Custom|LoadPlayerState
  (params (Player%20Progress :type Save%20Player%20Progress%20Object%20Reference))
  (bind _playerstate (Variables|/Game/Blueprints/Level_Save_Checkpoint_Logic/SavePlayerProgress.SavePlayerProgress_C|GetPlayerState Player%20Progress))
  ;[1 1 1] Load Player State
  (bind _outactors (Actor|GetAllActorswithTag "Player"))
  (for _array_element _outactors
    (bind _ascube_game_character (Utilities|Casting|CastToCubeGameCharacter _array_element))
    (Transformation|SetActorTransform _ascube_game_character (.playerposition _playerstate))
    (Development|PrintString (Utilities|String|Append "Set Actor Transform :" (Utilities|String|ToString(Transform) (.playerposition _playerstate))) true true "(R=0.000000,G=0.660000,B=1.000000,A=1.000000)" 5.0)
    (Variables|/Game/Blueprints/Items/InventoryComponent.InventoryComponent_C|SetInventory (Variables|/Game/Blueprints/CubeGameCharacter.CubeGameCharacter_C|GetInventoryComponent _ascube_game_character) (.playerinventory _playerstate))
    (Default|CallInventoryChangedDispatcher (Variables|/Game/Blueprints/CubeGameCharacter.CubeGameCharacter_C|GetInventoryComponent _ascube_game_character))))

(event Custom|LoadLevelState
  (params (Player%20Progress :type Save%20Player%20Progress%20Object%20Reference))
  (bind _levelstate (Variables|/Game/Blueprints/Level_Save_Checkpoint_Logic/SavePlayerProgress.SavePlayerProgress_C|GetLevelState Player%20Progress))
  ;[1 1 1] Load Level State
  (Development|PrintString "Open Level")
  (Development|PrintString (.levelname _levelstate))
  (Game|OpenLevel(byName) (Utilities|String|StringToName (.levelname _levelstate)))
  (bind _outactors (Actor|GetAllActorswithTag "Transportable"))
  (for _array_element _outactors
    (Actor|DestroyActor _array_element))
  (for _array_element_2 (.cubepositions _levelstate)
    (Game|SpawnActorfromClass "/Game/Cubes/Transportable.Transportable_C" _array_element_2 "Undefined" 0 0)))

(event Custom|LoadGameSave
  (params (DestroyedActor :type Actor%20Object%20Reference))
  ;[1 1 1] LoadGameSave
  (Development|PrintString "Try Load Savefile")
  (bind _returnvalue (SaveGame|LoadGamefromSlot (Variables|Default|GetGame%20Save%20Slot)))
  (bind _assave_player_progress (Utilities|Casting|CastToSavePlayerProgress _returnvalue))
  (CallFunction|LoadLevelState _assave_player_progress)
  (CallFunction|LoadPlayerState _assave_player_progress))

(fn ConstructionScript
  (Components|Box|SetBoxExtent (Variables|Default|GetLoadTrigger) (Variables|Default|GetResizeTriggerVolume) true))